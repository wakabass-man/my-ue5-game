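; BP_RoomGenerator is a legacy procedural room generator that builds a chain of rooms, starting from a BP_RushRoom spawned on BeginPlay.
; SpawnRandomRoom picks a random class from RoomArray and spawns it at the world transform of the first child component under the latest room's ExitFolder.
; Each spawned room becomes LastestRoom, so the next one attaches to its exit.
; Nothing in this graph calls SpawnRandomRoom.
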(event `self.ReceiveBeginPlay`
  (bind _returnvalue (`|SpawnActorFromClass` "/Game/Mine/ProceduralRoom/Legacy/Rooms/ChildrenRooms/BP_RushRoom.BP_RushRoom_C" (`KismetMathLibrary.MakeTransform` (0.0 0.0 0.0)) "Undefined" "MultiplyWithRoot" null null))
  (set `self.LastestRoom` _returnvalue))

(event `SpawnRandomRoom`
  (bind _returnvalue (`|SpawnActorFromClass` (`KismetArrayLibrary.Array_Random` (`self.RoomArray`)) (`SceneComponent.K2_GetComponentToWorld` (`SceneComponent.GetChildComponent` (`/Game/Mine/ProceduralRoom/Legacy/Rooms/ParentsRoom/BP_MasterRoom.ExitFolder` (`self.LastestRoom`)) 0)) "Undefined" "MultiplyWithRoot" null null))
  (set `self.LastestRoom` _returnvalue))

(fn `UserConstructionScript`)