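; BP_ForwardRoom is a child room Blueprint in the legacy procedural room system.
; When an overlap with its RoomSpawnTrigger ends, it finds the BP_RoomGenerator in the level and calls SpawnRandomRoom.
; It then destroys the overlapped trigger component, so each room requests a new room only once.
; BeginPlay, ActorBeginOverlap and construction defer to the parent class, and Tick is disabled.
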(event `self.ReceiveBeginPlay`
  (`parent.ReceiveBeginPlay`))

(event `self.ReceiveActorBeginOverlap`
  (params (OtherActor :type "Actor Object Reference"))
  (`parent.ReceiveActorBeginOverlap` OtherActor))

(event `self.RoomSpawnTrigger.OnComponentEndOverlap`
  (params (OverlappedComponent :type "PrimitiveComponent Object Reference") (OtherActor :type "Actor Object Reference") (OtherComp :type "PrimitiveComponent Object Reference") (OtherBodyIndex :type Integer))
  (bind _returnvalue (`GameplayStatics.GetActorOfClass` "/Game/Mine/ProceduralRoom/Legacy/BP_RoomGenerator.BP_RoomGenerator_C"))
  (`/Game/Mine/ProceduralRoom/Legacy/BP_RoomGenerator.SpawnRandomRoom` _returnvalue)
  (`ActorComponent.K2_DestroyComponent` OverlappedComponent))

(fn `UserConstructionScript`
  (`parent.UserConstructionScript`))