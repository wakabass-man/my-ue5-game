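; BP_RushWallExternalStrainField is a physics field actor that applies external cluster strain for breaking a rush wall's destructible geometry.
; DestructionRushWall feeds a radial falloff node, sized and centered on the Sphere component with no falloff, into the field system using the FieldMagnitude variable.
; It runs from the construction script, so the field fires on construction, and prints a debug string; the event graph is empty.
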(fn `DestructionRushWall`
  (bind _sphere (`self.Sphere`))
  (`FieldSystemComponent.ApplyPhysicsField` (`self.FieldSystemComponent`) true "Field_ExternalClusterStrain" null (`RadialFalloff.SetRadialFalloff` (`self.RadialFalloffComponent`) (`self.Field Magnitude`) 0.0 1.0 0.0 (`SphereComponent.GetScaledSphereRadius` _sphere) (`SceneComponent.K2_GetComponentLocation` _sphere) "Field_FallOff_None"))
  (`KismetSystemLibrary.PrintString` "External Strain"))

(fn `UserConstructionScript`
  (`self.DestructionRushWall`))