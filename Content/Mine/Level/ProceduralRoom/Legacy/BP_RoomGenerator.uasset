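; BP_RoomGenerator is an actor that builds a level by chaining procedural rooms, each with a coin pickup.
; BeginPlay spawns a starting BP_RushRoom and stores it as the latest room.
; SpawnRandomRoom spawns a random class from RoomArray at the latest room's first ExitFolder component transform, then makes it the latest.
; Each room gets a half-scale BP_Coin placed slightly above its first CollisionFolder component.
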(event `self.ReceiveBeginPlay`
  (bind _returnvalue (`|SpawnActorFromClass` "/Game/Mine/Level/ProceduralRoom/Legacy/Rooms/ChildrenRooms/BP_RushRoom.BP_RushRoom_C" (`KismetMathLibrary.MakeTransform` (0.0 0.0 0.0)) "Undefined" "MultiplyWithRoot" null null))
  (bind _output_get (set `self.LastestRoom` _returnvalue))
  (bind _returnvalue_2 (`SceneComponent.K2_GetComponentToWorld` (`SceneComponent.GetChildComponent` (`/Game/Mine/Level/ProceduralRoom/Legacy/Rooms/ParentsRoom/BP_MasterRoom.CollisionFolder` _output_get) 0)))
  (`|SpawnActorFromClass` "/Game/Mine/Items/FieldItems/BP_Coin.BP_Coin_C" (`KismetMathLibrary.MakeTransform` (`KismetMathLibrary.MakeVector` (.x (.location _returnvalue_2)) (.y (.location _returnvalue_2)) (+ (.z (.location _returnvalue_2)) 100.0)) (struct) (0.5 0.5 0.5)) "Undefined" "MultiplyWithRoot" null null))

(event `SpawnRandomRoom`
  (bind _returnvalue (`|SpawnActorFromClass` (`KismetArrayLibrary.Array_Random` (`self.RoomArray`)) (`SceneComponent.K2_GetComponentToWorld` (`SceneComponent.GetChildComponent` (`/Game/Mine/Level/ProceduralRoom/Legacy/Rooms/ParentsRoom/BP_MasterRoom.ExitFolder` (`self.LastestRoom`)) 0)) "Undefined" "MultiplyWithRoot" null null))
  (set `self.LastestRoom` _returnvalue)
  (bind _returnvalue_2 (`SceneComponent.K2_GetComponentToWorld` (`SceneComponent.GetChildComponent` (`/Game/Mine/Level/ProceduralRoom/Legacy/Rooms/ParentsRoom/BP_MasterRoom.CollisionFolder` _returnvalue) 0)))
  (`|SpawnActorFromClass` "/Game/Mine/Items/FieldItems/BP_Coin.BP_Coin_C" (`KismetMathLibrary.MakeTransform` (`KismetMathLibrary.MakeVector` (.x (.location _returnvalue_2)) (.y (.location _returnvalue_2)) (+ (.z (.location _returnvalue_2)) 100.0)) (struct) (0.5 0.5 0.5)) "Undefined" "MultiplyWithRoot" null null))

(fn `UserConstructionScript`)