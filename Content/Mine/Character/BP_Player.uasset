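; Player character Blueprint that picks up items and punches with Chaos field effects.
; On BeginPlay it creates the inventory widget and a hidden crosshair; capsule overlap with a BaseItem updates the inventory and destroys the item.
; Punch_1 calls SpawnStrainField, which debug-traces from the left thumb bone toward a point ahead of the follow camera and spawns an external strain field at the impact point.
; A master field spawn is left unconnected.
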(event `self.CapsuleComponent.OnComponentBeginOverlap`
  (params (OverlappedComponent :type "PrimitiveComponent Object Reference") (OtherActor :type "Actor Object Reference") (OtherComp :type "PrimitiveComponent Object Reference") (OtherBodyIndex :type Integer) (bFromSweep :type Boolean) (SweepResult :type "HitResult Structure (by ref)"))
  ;[1 1 1 1 22] 아이템 먹기
  (bind _asbase_item (cast `BaseItem` OtherActor))
  (`/Game/Mine/UI/WB_Inventory.UpdateInventory` (`self.InventoryWidget`) _asbase_item)
  (`self.K2_DestroyActor` _asbase_item))

(event `self.ReceiveTick`
  (params (DeltaSeconds :type "Float (single-precision)")))

(event `self.ReceiveBeginPlay`
  ;[1 1 1 1 22] 비긴 플레이시 위젯 세팅
  (bind _returnvalue (`|CreateWidget` "/Game/Mine/UI/WB_Inventory.WB_Inventory_C"))
  (bind _output_get (set `self.InventoryWidget` _returnvalue))
  (`UserWidget.AddToViewport` _output_get 0)
  (bind _returnvalue_2 (`|CreateWidget` "/Game/Mine/UI/WB_CrossHair.WB_CrossHair_C"))
  (bind _output_get_2 (set `self.CrossHairWidget` _returnvalue_2))
  (`UserWidget.AddToViewport` _output_get_2 0)
  (`Widget.SetVisibility` _output_get_2 "Hidden"))

(event `Punch_1`
  (params (Value :type "InputActionValue Structure (by ref)"))
  (bind _followcamera (`self.FollowCamera`))
  (bind _returnvalue_location (`KismetMathLibrary.BreakTransform` (`SkinnedMeshComponent.GetBoneTransform` (`self.Mesh`) "thumb_03_l" "RTS_World")))
  (bind _outhit (`KismetSystemLibrary.LineTraceSingle` :`Start` _returnvalue_location :`End` (+ (`SceneComponent.K2_GetComponentLocation` _followcamera) (* (`SceneComponent.GetForwardVector` _followcamera) 1000.0)) :`TraceChannel` "TraceTypeQuery1" :`DrawDebugType` "ForDuration" :`TraceColor` (struct :`G` 1.0 :`B` 0.112953 :`A` 1.0) :`TraceHitColor` (struct :`R` 1.0 :`G` 0.009645 :`A` 1.0) :`DrawTime` 3.0))
  (`|SpawnActorFromClass` "/Game/Mine/Physics/FS_PunchExternalStrainField.FS_PunchExternalStrainField_C" (`KismetMathLibrary.MakeTransform` (`.ImpactPoint` (`GameplayStatics.BreakHitResult` _outhit)) (struct) (3.0 3.0 3.0)) "AlwaysSpawn" "MultiplyWithRoot" null null))

(fn `UserConstructionScript`)